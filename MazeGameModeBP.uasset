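; Game mode for a maze game that manages level progression, lives, the HUD and music.
; On BeginPlay it loads or creates the save game, finds the current map in the Levels array and records the highest level reached.
; Functions handle restarting, advancing, returning to the menu, unpausing and changing lives, with life changes saved immediately.
; Restart and menu exit reset progress and lives when none remain.
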(event Custom|SaveLevel
  (bind _returnvalue (SaveGame|DoesSaveGameExist "save1"))
  (if _returnvalue
    (bind _returnvalue_2 (SaveGame|LoadGamefromSlot "save1"))
    (bind _asmaze_save_game_bp (Utilities|Casting|CastToMazeSaveGameBP _returnvalue_2))
    (Variables|Default|SetSaver _asmaze_save_game_bp)
    (else
      (bind _returnvalue_3 (SaveGame|CreateSaveGameObject "/Game/MazeSaveGameBP.MazeSaveGameBP_C"))
      (Variables|Default|SetSaver _returnvalue_3)))
  (bind (_array_element _array_index) (Utilities|Array|ForEachLoopwithBreak (Variables|Default|GetLevels) :!label _label)
    (:LoopBody
      (bind _returnvalue_4 (Game|GetCurrentLevelName true))
      (if (== _array_element _returnvalue_4)
        (Utilities|FlowControl|Sequence
          (:then_0
            (Variables|Default|SetLevel _array_index))
          (:then_1
            (if (> _array_index (Variables|/Game/MazeSaveGameBP.MazeSaveGameBP_C|GetHighest%20Level (Variables|Default|GetSaver)))
              (Variables|/Game/MazeSaveGameBP.MazeSaveGameBP_C|SetHighest%20Level (Variables|Default|GetSaver) _array_index)))
          (:then_2
            (goto _label Break)))))
    (:Completed
      (SaveGame|SaveGametoSlot (Variables|Default|GetSaver) "save1"))))

(event EventBeginPlay
  (bind _returnvalue (UserInterface|CreateWidget "/Game/UI/HUD.HUD_C"))
  (UserInterface|Viewport|AddtoViewport _returnvalue 0)
  (Variables|/Script/Engine.PlayerController|SetbShowMouseCursor (Game|GetPlayerController 0) false)
  (CallFunction|SaveLevel)
  (Audio|PlaySound2D "/Game/Audio/MainSong.MainSong" 1.0 1.0 0.0 "/Game/Audio/MusicConcurrent.MusicConcurrent" 0))

(event EventTick
  (params (DeltaSeconds :type Float%20%28single-precision%29)))

(fn ConstructionScript)

(fn RestartLevel
  (bind _saver (Variables|Default|GetSaver))
  (if (> (Variables|/Game/MazeSaveGameBP.MazeSaveGameBP_C|GetLives _saver) 0)
    _
    (else
      (bind _output_get (Variables|Default|SetLevel 0))
      (Variables|/Game/MazeSaveGameBP.MazeSaveGameBP_C|SetHighest%20Level _saver _output_get)
      (Variables|/Game/MazeSaveGameBP.MazeSaveGameBP_C|SetLives _saver 3)
      (SaveGame|SaveGametoSlot (Variables|Default|GetSaver) "save1")))
  (Game|OpenLevel(byName) (Utilities|Array|Get(acopy) (Variables|Default|GetLevels) (Variables|Default|GetLevel))))

(fn MainMenu
  (params (Won%20Level :type Boolean))
  (bind _saver (Variables|Default|GetSaver))
  (bind _saver_2 (Variables|Default|GetSaver))
  (if Won%20Level
    (bind _output_get (Variables|Default|SetLevel (+ (stale _output_get) 1)))
    (Variables|/Game/MazeSaveGameBP.MazeSaveGameBP_C|SetHighest%20Level _saver _output_get))
  (Utilities|FlowControl|Sequence
    (:then_0
      (if (> (Variables|/Game/MazeSaveGameBP.MazeSaveGameBP_C|GetLives _saver) 0)
        _
        (else
          (bind _output_get_2 (Variables|Default|SetLevel 0))
          (Variables|/Game/MazeSaveGameBP.MazeSaveGameBP_C|SetHighest%20Level _saver_2 _output_get_2)
          (Variables|/Game/MazeSaveGameBP.MazeSaveGameBP_C|SetLives _saver_2 3)))
      (SaveGame|SaveGametoSlot _saver_2 "save1"))
    (:then_1
      (Game|OpenLevel(byName) "Menu"))))

(fn NextLevel
  (bind _levels (Variables|Default|GetLevels))
  (bind _result (Math|Integer|IncrementInt (Variables|Default|GetLevel))
    (:%20%20
      (if (>= _result (Utilities|Array|Length _levels))
        (CallFunction|MainMenu false)
        (else
          (Game|OpenLevel(byName) (Utilities|Array|Get(acopy) _levels _result)))))))

(fn BacktoGame
  (Viewport|RemoveAllWidgets)
  (bind _returnvalue (UserInterface|CreateWidget "/Game/UI/HUD.HUD_C"))
  (UserInterface|Viewport|AddtoViewport _returnvalue 0)
  (Variables|/Script/Engine.PlayerController|SetbShowMouseCursor (Game|GetPlayerController 0) false)
  (Game|SetGamePaused false))

(fn ExtraLife
  (bind _saver (Variables|Default|GetSaver))
  (Math|Integer|IncrementInt (Variables|/Game/MazeSaveGameBP.MazeSaveGameBP_C|GetLives _saver)
    (:%20%20
      (SaveGame|SaveGametoSlot _saver "save1"))))

(fn RemoveLife
  (bind _saver (Variables|Default|GetSaver))
  (bind _output_get (Variables|/Game/MazeSaveGameBP.MazeSaveGameBP_C|SetLives _saver (- (stale _output_get) 1)))
  (SaveGame|SaveGametoSlot _saver "save1"))