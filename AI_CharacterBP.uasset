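; AI enemy character Blueprint that scans its surroundings and can launch grenade projectiles.
; On Tick it asks its EnemyController whether it can see the player, and while it cannot, it spins around its yaw at LookSpeed, scaled by delta time.
; ShootProj, which is not called within this Blueprint, spawns a GrenadeBP above the actor and applies a forward impulse to its Sphere.
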(event EventBeginPlay)

(event Collision|EventActorBeginOverlap
  (params (OtherActor :type Actor%20Object%20Reference)))

(event EventTick
  (params (DeltaSeconds :type Float%20%28single-precision%29))
  (bind _returnvalue (Transformation|GetActorRotation))
  (bind _asenemy_controller (Utilities|Casting|CastToEnemyController (Pawn|GetController)))
  (bind _cansee (Default|CanSeePlayer _asenemy_controller))
  (if (not _cansee)
    (Transformation|SetActorRotation (Math|Rotator|MakeRotator (.roll _returnvalue) (.pitch _returnvalue) (+ (.yaw _returnvalue) (* DeltaSeconds (Variables|Default|GetLookSpeed)))))))

(fn ConstructionScript)

(fn ShootProj
  (bind _returnvalue (Game|SpawnActorfromClass "/Game/GrenadeBP.GrenadeBP_C" (Math|Transform|MakeTransform (+ (Transformation|GetActorLocation) (* (Math|Vector|VectorUp) 1.5e+02)) (Transformation|GetActorRotation) "1.000000,1.000000,1.000000") "Undefined" "MultiplyWithRoot" 0 0))
  (Physics|AddImpulse (Variables|/Game/GrenadeBP.GrenadeBP_C|GetSphere _returnvalue) (* (Transformation|GetActorForwardVector) 2e+03) "None" false))